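; BottomWin is a win trigger that declares a race result when an actor overlaps it, presumably for the bottom player.
; On BeginPlay it sets Order to -1, runs parent logic, then hides itself and disables collision, so it stays inert until re-enabled outside this Blueprint.
; Any overlap, without filtering the actor, finds Player1 and calls DeclareWinner(false) on its CheckpointManagerForBothPlayers.
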(event `self.ReceiveBeginPlay`
  (set `self.Order` -1)
  (`parent.ReceiveBeginPlay`)
  (`self.SetActorHiddenInGame` true)
  (`self.SetActorEnableCollision` false))

(event `self.ReceiveActorBeginOverlap`
  (params (OtherActor :type "Actor Object Reference"))
  (`parent.ReceiveActorBeginOverlap` OtherActor)
  (bind _returnvalue (`GameplayStatics.GetActorOfClass` "/Game/Blueprints/Player1.Player1_C"))
  (`/Game/Blueprints/CheckpointManager.DeclareWinner` (`/Game/Blueprints/Player1.CheckpointManagerForBothPlayers` _returnvalue) false))

(fn `UserConstructionScript`
  (`parent.UserConstructionScript`))