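; Sets up two-player local play at BeginPlay by spawning and possessing a pawn for each player.
; Loops over all PlayerStarts, reads each tag as an integer, and spawns at that start's X/Y, rotation and scale.
; Tag 0 goes to player controller 0; tag 1 creates a second local player to possess a Player2 pawn, rolled 180 degrees to spawn upside down.
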(event `self.ReceiveBeginPlay`
  (bind _outactors (`GameplayStatics.GetAllActorsOfClass` "/Script/Engine.PlayerStart"))
  (for _array_element _outactors
    (switch `int` (`KismetStringLibrary.Conv_StringToInt` (`KismetStringLibrary.Conv_NameToString` (`PlayerStart.PlayerStartTag` _array_element)))
      (:`0`
        (bind _returnvalue (`self.GetTransform` _array_element))
        (bind _returnvalue_2 (`|SpawnActorFromClass` "/Game/Blueprints/Player1.Player1_C" (`KismetMathLibrary.MakeTransform` (`KismetMathLibrary.MakeVector` (.x (.location _returnvalue)) (.y (.location _returnvalue))) (`KismetMathLibrary.MakeRotator` (.roll (.rotation _returnvalue)) (.pitch (.rotation _returnvalue)) (.yaw (.rotation _returnvalue))) (.scale _returnvalue)) "AdjustIfPossibleButAlwaysSpawn" "OverrideRootScale" null null))
        (`Controller.Possess` (`GameplayStatics.GetPlayerController` 0) _returnvalue_2))
      (:`1`
        (bind _returnvalue_3 (`GameplayStatics.CreatePlayer` -1))
        (bind _returnvalue_4 (`|SpawnActorFromClass` "/Game/Blueprints/Player2.Player2_C" (`KismetMathLibrary.MakeTransform` (`KismetMathLibrary.MakeVector` (.x (.location _returnvalue)) (.y (.location _returnvalue))) (`KismetMathLibrary.MakeRotator` (+ (.roll (.rotation _returnvalue)) 180.0) (.pitch (.rotation _returnvalue)) (.yaw (.rotation _returnvalue))) (.scale _returnvalue)) "AdjustIfPossibleButAlwaysSpawn" "OverrideRootScale" null null))
        (`Controller.Possess` _returnvalue_3 _returnvalue_4)))))

(fn `UserConstructionScript`)