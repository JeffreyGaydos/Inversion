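; Player1 vehicle pawn that also relays the second player's driving controls to the Player2 vehicle.
; On BeginPlay it finds the Player2 actor and forwards the second set of throttle, steering and handbrake inputs to that vehicle's movement component.
; Each tick it applies a fake gravity Z force to its own mesh, computed from mesh mass and FakeGravity divided by delta time.
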(event `InputAxis|MoveRight2`
  (params (AxisValue :type "Float (single-precision)"))
  (`WheeledVehicleMovementComponent.SetSteeringInput` (`WheeledVehicle.VehicleMovement` (`self.Player2`)) AxisValue))

(event `self.ReceiveBeginPlay`
  (`parent.ReceiveBeginPlay`)
  (bind _returnvalue (`GameplayStatics.GetActorOfClass` "/Game/Blueprints/Player2.Player2_C"))
  (set `self.Player2` _returnvalue))

(event `InputAxis|MoveForward2`
  (params (AxisValue :type "Float (single-precision)"))
  (`WheeledVehicleMovementComponent.SetThrottleInput` (`WheeledVehicle.VehicleMovement` (`self.Player2`)) AxisValue))

(event `self.ReceiveTick`
  (params (DeltaSeconds :type "Float (single-precision)"))
  (`parent.ReceiveTick` DeltaSeconds)
  (bind (_mesh _zforce) (`self.CalculateFakeGravity` DeltaSeconds))
  (`PrimitiveComponent.AddForce` _mesh (`KismetMathLibrary.MakeVector` 0.0 0.0 _zforce) "None" false))

(event `InputAction|Handbrake2`
  (params (Key :type "Key Structure"))
  (bind _vehiclemovement (`WheeledVehicle.VehicleMovement` (`self.Player2`)))
  (:`Pressed`
    (`WheeledVehicleMovementComponent.SetHandbrakeInput` _vehiclemovement true))
  (:`Released`
    (`WheeledVehicleMovementComponent.SetHandbrakeInput` _vehiclemovement false)))

(fn `CalculateFakeGravity`
  (params (deltaTime :type "Float (double-precision)"))
  (returns (Mesh :type "SkeletalMeshComponent Object Reference") (ZForce :type "Float (double-precision)"))
  (bind _mesh (`self.Mesh`))
  (return _mesh (* (`PrimitiveComponent.GetMass` _mesh) (/ (`self.FakeGravity`) deltaTime))))

(fn `UserConstructionScript`
  (`parent.UserConstructionScript`))