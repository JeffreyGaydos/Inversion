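; Player2 is a child vehicle pawn for what appears to be the second player, driven by a custom fake gravity.
; Empty MoveForward and MoveRight axis events override the parent's input bindings.
; Each tick applies a Z force of mass times FakeGravity over delta time to both Mesh and the movement component's updated primitive.
; It calls Respawn when the mesh's Z is above KillZ, otherwise prints KillZ.
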(event `self.ReceiveBeginPlay`
  (`parent.ReceiveBeginPlay`))

(event `InputAxis|MoveForward`
  (params (AxisValue :type "Float (single-precision)"))
  ;[1 1 1] Required to override the parent bindings and force the new ones
)

(event `InputAxis|MoveRight`
  (params (AxisValue :type "Float (single-precision)"))
  ;[1 1 1] Required to override the parent bindings and force the new ones
)

(event `InputAction|Handbrake`
  (params (Key :type "Key Structure"))
  ;[1 1 1] Required to override the parent bindings and force the new ones
)

(event `self.ReceiveTick`
  (params (DeltaSeconds :type "Float (single-precision)"))
  (bind _mesh (`self.Mesh`))
  (bind _killz (`self.KillZ`))
  (bind (_returnvalue_x _returnvalue_y _returnvalue_z) (`KismetMathLibrary.BreakVector` (`SceneComponent.K2_GetComponentLocation` (`self.Mesh`))))
  (`parent.ReceiveTick` DeltaSeconds)
  (bind _zforce (`self.CalculateFakeGravity` DeltaSeconds _mesh))
  (`PrimitiveComponent.AddForce` _mesh (`KismetMathLibrary.MakeVector` 0.0 0.0 _zforce) "None" false)
  (`PrimitiveComponent.AddForce` (`MovementComponent.UpdatedPrimitive` (`self.VehicleMovement`)) (`KismetMathLibrary.MakeVector` 0.0 0.0 _zforce) "None" false)
  (if (> _returnvalue_z _killz)
    (`/Game/Blueprints/IPlayer.Respawn`)
    (else
      (`KismetSystemLibrary.PrintString` (`KismetStringLibrary.Conv_DoubleToString` _killz)))))

(fn `CalculateFakeGravity`
  (params (deltaTime :type "Float (double-precision)") (SelfMesh :type "PrimitiveComponent Object Reference"))
  (returns (ZForce :type "Float (double-precision)"))
  (return (* (`PrimitiveComponent.GetMass` SelfMesh) (/ (`self.FakeGravity`) deltaTime))))

(fn `UserConstructionScript`
  (`parent.UserConstructionScript`))