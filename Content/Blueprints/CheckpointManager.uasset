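; Checkpoint manager for a two-player race, running separate upper and lower checkpoint sequences and declaring the first winner.
; At BeginPlay it gathers each track's checkpoints, sorts them by Order with nested loops, hides them and activates each track's first.
; ActivateCheckpoint reveals and enables the requested checkpoint, or that player's win point once the index reaches the list's end.
; DeclareWinner shows the win widget and mouse cursor, guarded to run once.
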(event `self.ReceiveBeginPlay`
  (bind _lowercpordered (`self.LowerCPOrdered`))
  (bind _outactors (`GameplayStatics.GetAllActorsOfClass` "/Game/Blueprints/Checkpoint.Checkpoint_C"))
  (bind _output_get (set `self.UpperCheckpoitns` _outactors))
  (`self.PopulateOrderedArraysTop` _output_get (`self.UpperCPOrdered`))
  (bind _outactors_2 (`GameplayStatics.GetAllActorsOfClass` "/Game/Blueprints/CHeckpointBottom.CHeckpointBottom_C"))
  (bind _output_get_2 (set `self.LowerCheckpoints` _outactors_2))
  (`self.PopulateOrderedArraysBottom` _output_get_2 _lowercpordered)
  (`KismetSystemLibrary.PrintString` (`KismetStringLibrary.Conv_IntToString` (`KismetArrayLibrary.Array_Length` _lowercpordered)))
  (`self.ActivateCheckpoint` 0)
  (`self.ActivateCheckpoint` 0 true))

(event `self.ReceiveTick`
  (params (DeltaSeconds :type "Float (single-precision)")))

(fn `ActivateCheckpoint`
  (params (CheckpointIndex :type Integer) (Player1 :type Boolean))
  (bind _uppercpordered (`self.UpperCPOrdered`))
  (bind _lowercpordered (`self.LowerCPOrdered`))
  (if Player1
    (if (== CheckpointIndex (`KismetArrayLibrary.Array_Length` _uppercpordered))
      (`self.ActivateWinpoint` true)
      (else
        (for (_array_element _array_index) _uppercpordered
          (if (== _array_index CheckpointIndex)
            (`Actor.SetActorHiddenInGame` _array_element false)
            (`Actor.SetActorEnableCollision` _array_element true)))))
    (elif (== (`KismetArrayLibrary.Array_Length` _lowercpordered) CheckpointIndex)
      (`self.ActivateWinpoint` false)
      (else
        (for (_array_element_2 _array_index_2) _lowercpordered
          (if (== _array_index_2 CheckpointIndex)
            (`Actor.SetActorHiddenInGame` _array_element_2 false)
            (`Actor.SetActorEnableCollision` _array_element_2 true)))))))

(fn `ActivateWinpoint`
  (params (Player1 :type Boolean))
  (if Player1
    (bind _returnvalue (`GameplayStatics.GetActorOfClass` "/Game/Blueprints/TopWin.TopWin_C"))
    (else
      (bind _returnvalue_2 (`GameplayStatics.GetActorOfClass` "/Game/Blueprints/BottomWin.BottomWin_C"))))
  (`Actor.SetActorHiddenInGame` _returnvalue false)
  (`Actor.SetActorHiddenInGame` _returnvalue_2 false)
  (`Actor.SetActorEnableCollision` _returnvalue_2 true)
  (`Actor.SetActorEnableCollision` _returnvalue true))

(fn `DeclareWinner`
  (params (WinnerPlayer1 :type Boolean))
  (if (not (`self.WinnerFound`))
    (set `self.WinnerFound` true)
    (bind _returnvalue (`|CreateWidget` "/Game/Menus/Win.Win_C"))
    (`/Game/Menus/Win.SetWinText` _returnvalue WinnerPlayer1)
    (`UserWidget.AddToViewport` _returnvalue 0)
    (set `PlayerController.bShowMouseCursor` true (`GameplayStatics.GetPlayerController` 0))))

(fn `PopulateOrderedArraysBottom`
  (params (CheckpointActors :type "Array of /Game/Blueprints/CHeckpointBottom Object Reference") (OrderedCheckpointArray :type "Array of /Game/Blueprints/CHeckpointBottom Object Reference"))
  (for (_ _array_index) CheckpointActors
    (for _array_element CheckpointActors
      (cast `/Game/Blueprints/BottomWin` _array_element
        (:`CastFailed`
          (if (== _array_index (`/Game/Blueprints/Checkpoint.Order` _array_element))
            (`KismetArrayLibrary.Array_Add` OrderedCheckpointArray _array_element)
            (`Actor.SetActorHiddenInGame` _array_element true)
            (`Actor.SetActorEnableCollision` _array_element false)))))))

(fn `PopulateOrderedArraysTop`
  (params (CheckpointActors :type "Array of /Game/Blueprints/Checkpoint Object Reference") (OrderedCheckpointArray :type "Array of /Game/Blueprints/Checkpoint Object Reference"))
  (for (_ _array_index) CheckpointActors
    (for _array_element CheckpointActors
      (cast `/Game/Blueprints/CHeckpointBottom` _array_element
        (:`CastFailed`
          (if (== _array_index (`/Game/Blueprints/Checkpoint.Order` _array_element))
            (`KismetArrayLibrary.Array_Add` OrderedCheckpointArray _array_element)
            (`Actor.SetActorHiddenInGame` _array_element true)
            (`Actor.SetActorEnableCollision` _array_element false)))))))