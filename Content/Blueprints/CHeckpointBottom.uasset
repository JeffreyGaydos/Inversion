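; Checkpoint actor, the bottom variant, that updates the respawn point of a Player2 that overlaps it.
; On overlap it passes its location and rotation to the player's SetRespawnMessage, with roll flipped 180 degrees and yaw offset by a quarter turn.
; It then plays the checkpoint sound at its scene location and destroys its Cube component, leaving the actor itself in place.
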(event `self.ReceiveBeginPlay`
  (`parent.ReceiveBeginPlay`))

(event `self.ReceiveActorBeginOverlap`
  (params (OtherActor :type "Actor Object Reference"))
  (bind _returnvalue (`self.GetTransform` self))
  (bind _asplayer_2 (cast `/Game/Blueprints/Player2` OtherActor))
  (message `/Game/Blueprints/IPlayer.SetRespawn` _asplayer_2 (`KismetMathLibrary.MakeTransform` (.location _returnvalue) (`KismetMathLibrary.MakeRotator` (+ (.roll (.rotation _returnvalue)) 180.0) (.pitch (.rotation _returnvalue)) (+ (.yaw (.rotation _returnvalue)) -90.0))))
  (`GameplayStatics.PlaySoundAtLocation` "/Game/Sounds/Checkpoint.Checkpoint" (`SceneComponent.K2_GetComponentLocation` (`self.Scene`)) (struct) 3.0 1.0 0.0 null null null)
  (`ActorComponent.K2_DestroyComponent` (`self.Cube`)))

(fn `UserConstructionScript`
  (`parent.UserConstructionScript`))